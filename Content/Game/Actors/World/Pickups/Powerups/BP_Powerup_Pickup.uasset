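; Powerup pickup actor that grants the collecting user a character ability.
; When handling a pickup, it gives the configured AbilityToGive to the user and activates it immediately.
; On BeginPlay, it validates that ability class and, if none is set, prints an error and disables its own collision.
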(event `self.ReceiveBeginPlay`
  (if (not (`KismetSystemLibrary.IsValidClass` (`self.AbilityToGive`)))
    (`KismetSystemLibrary.PrintString` (`KismetStringLibrary.Concat_StrStr` "ERROR: " (`KismetSystemLibrary.GetDisplayName` self) " will not have it's collision enabled as there is no ability to give!") false)
    (`self.SetActorEnableCollision` false)))

(event `self.BlueprintHandlePickup`
  (params (ForUser :type "GridironCharacter Object Reference"))
  (`GridironCharacter.GiveCharacterAbility` ForUser (`self.AbilityToGive`) true))

(fn `UserConstructionScript`)