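; Weapon pickup Blueprint that grants the configured WeaponToAdd class to the user who picks it up.
; Its construction script fills the mesh and text label from that class's defaults, using the first-person mesh asset on Mesh3P.
; Pickup is always allowed, and users who already own the weapon receive its starting ammo instead of a duplicate.
; An invalid class prints an error on BeginPlay and disables the actor's collision.
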(event `self.ReceiveBeginPlay`
  (if (not (`KismetSystemLibrary.IsValidClass` (`self.WeaponToAdd`)))
    (`KismetSystemLibrary.PrintString` (`KismetStringLibrary.Concat_StrStr` "ERROR: " (`KismetSystemLibrary.GetDisplayName` self) " will not spawn its pickup class because the WeaponToAdd class is invalid. Please add a class for this to use!") false)
    (`self.SetActorEnableCollision` false)))

(event `self.BlueprintHandlePickup`
  (params (ForUser :type "GridironCharacter Object Reference"))
  (bind (_attachweaponsocketname _damagetypeclass _ammo _ammotype _ammopershot _minammorequiredtoshoot _bconsumesammo _startingammo) (defaults `Object` (`self.WeaponToAdd`)))
  (if (`GridironCharacter.HasItemInInventory` ForUser (`self.WeaponToAdd`))
    (`GridironCharacter.GiveAmmo` ForUser _ammotype _startingammo)
    (else
      (`GridironCharacter.AddItemToInventory` ForUser (`self.WeaponToAdd`)))))

(fn `BlueprintCanPickup`
  (params (ForUser :type "GridironCharacter Object Reference"))
  (returns (ReturnValue :type Boolean))
  (return true))

(fn `UserConstructionScript`
  (bind (_attachweaponsocketname _damagetypeclass _ammo _ammotype _ammopershot _minammorequiredtoshoot _bconsumesammo _startingammo _itemname _mesh1passet) (defaults `Object` (`self.WeaponToAdd`)))
  (if (`KismetSystemLibrary.IsValidClass` (`self.WeaponToAdd`))
    (`SkinnedMeshComponent.SetSkinnedAssetAndUpdate` (`self.Mesh3P`) _mesh1passet true)
    (`TextRenderComponent.K2_SetText` (`self.TextRender`) _itemname)))