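; GA_Slide is a Gameplay Ability that starts a slide on a GridironCharacter.
; Activation is gated by the character's CanSlide check, made on the owner actor.
; Once committed, it calls OnBeginSlide on the avatar character and ends immediately, leaving the slide itself to the character.
; A failed commit or cast ends the ability without sliding.
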(event `self.K2_ActivateAbility`
  (bind _returnvalue (`self.K2_CommitAbility`))
  (if _returnvalue
    (bind _asgridiron_character (cast `GridironCharacter` (`self.GetAvatarActorFromActorInfo`))
      (:`then`
        (`GridironCharacter.OnBeginSlide` _asgridiron_character))
      (:`CastFailed`
        _))
    (`self.K2_EndAbility`)
    (else
      (`self.K2_EndAbility`))))

(fn `K2_CanActivateAbility`
  (params (ActorInfo :type "GameplayAbilityActorInfo Structure"))
  (returns (RelevantTags :type "GameplayTagContainer Structure") (ReturnValue :type Boolean))
  (bind _asgridiron_character (cast `GridironCharacter` (`.OwnerActor` (break `GameplayAbilityActorInfo` ActorInfo)))
    (:`then`
      (return (struct) (`GridironCharacter.CanSlide` _asgridiron_character)))
    (:`CastFailed`
      (return (struct) false))))