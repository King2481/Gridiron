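; GA_Crouch is a hold-to-crouch gameplay ability for GridironCharacter avatars.
; Activation requires the owner to be a GridironCharacter whose CanCrouch returns true.
; After committing, it starts a WaitInputRelease task and crouches the avatar, then uncrouches and ends the ability when input is released.
; A failed commit ends the ability immediately, and the ability's end event does no cleanup.
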(event `self.K2_ActivateAbility`
  (bind _returnvalue (`self.GetAvatarActorFromActorInfo`))
  (bind _returnvalue_2 (`self.K2_CommitAbility`))
  (if _returnvalue_2
    (`AbilityTask_WaitInputRelease.WaitInputRelease` false
      (:`then`
        (bind _asgridiron_character (cast `GridironCharacter` _returnvalue))
        (`Character.Crouch` _asgridiron_character))
      (:`OnRelease`
        (bind _asgridiron_character_2 (cast `GridironCharacter` _returnvalue))
        (`Character.UnCrouch` _asgridiron_character_2)
        (`self.K2_EndAbility`)))
    (else
      (`self.K2_EndAbility`))))

(fn `K2_CanActivateAbility`
  (params (ActorInfo :type "GameplayAbilityActorInfo Structure"))
  (returns (RelevantTags :type "GameplayTagContainer Structure") (ReturnValue :type Boolean))
  (bind _asgridiron_character (cast `GridironCharacter` (`.OwnerActor` (break `GameplayAbilityActorInfo` ActorInfo)))
    (:`then`
      (return (struct) (`Character.CanCrouch` _asgridiron_character)))
    (:`CastFailed`
      (return (struct) false))))