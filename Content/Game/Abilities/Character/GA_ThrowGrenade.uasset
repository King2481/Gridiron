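; GA_ThrowGrenade is a Gameplay Ability that lets a Gridiron character throw a grenade.
; On activation it commits the ability, then only on authority fires a BP_GA_ThrownGrenadeProjectile from the character's camera location along its control rotation forward vector.
; The ability ends immediately afterward, and also ends when the commit fails, authority is absent or the avatar is not a GridironCharacter.
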(event `self.K2_ActivateAbility`
  (bind _returnvalue (`self.K2_CommitAbility`))
  (if _returnvalue
    (`self.K2_HasAuthority`
      (:`True`
        (bind _asgridiron_character (cast `GridironCharacter` (`self.GetAvatarActorFromActorInfo`))
          (:`then`
            (set `self.FiredProjectile` (`WeaponStatics.FireProjectile` _asgridiron_character "/Game/Game/Actors/Projectiles/BP_GA_ThrownGrenadeProjectile.BP_GA_ThrownGrenadeProjectile_C" (`GridironCharacter.GetCameraLocation` _asgridiron_character) (`KismetMathLibrary.GetForwardVector` (`Pawn.GetControlRotation` _asgridiron_character))))
            (`self.K2_EndAbility`))
          (:`CastFailed`
            (`self.K2_EndAbility` :!label _label))))
      (:`False`
        (goto _label)))
    (else
      (goto _label))))