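; Gameplay ability that performs a character dash which damages and knocks back characters it hits.
; After committing, it starts the dash on GridironMovementComponent, binds capsule hit events, waits a fixed delay, then ends the dash and ability.
; On the authority, a hit GridironCharacter takes heavy point damage with a dash damage type and is launched away and upward using the impact normal.
; The hit binding is never explicitly removed.
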(event `self.K2_ActivateAbility`
  (bind _returnvalue (`self.K2_CommitAbility`))
  (if _returnvalue
    (bind _ascharacter (cast `Character` (`self.GetAvatarActorFromActorInfo`))
      (:`then`
        (bind _asgridiron_movement_component (cast `GridironMovementComponent` (`Character.CharacterMovement` _ascharacter))
          (:`then`
            (`GridironMovementComponent.StartDash` _asgridiron_movement_component)
            (add `PrimitiveComponent.OnComponentHit` (`Character.CapsuleComponent` _ascharacter) (delegate `OnCapsuleHit`))
            (`KismetSystemLibrary.Delay` 0.75)
            (`GridironMovementComponent.EndDash` _asgridiron_movement_component)
            (`self.K2_EndAbility`))
          (:`CastFailed`
            (`self.K2_EndAbility` :!label _label))))
      (:`CastFailed`
        (goto _label)))
    (else
      (goto _label))))

(event `OnCapsuleHit`
  (params (HitComponent :type "PrimitiveComponent Object Reference") (OtherActor :type "Actor Object Reference") (OtherComp :type "PrimitiveComponent Object Reference") (NormalImpulse :type "Vector Structure") (Hit :type "HitResult Structure (by ref)"))
  (bind (_bblockinghit _binitialoverlap _time _distance _location _impactpoint _normal _impactnormal) (`GameplayStatics.BreakHitResult` Hit))
  (bind _asgridiron_character (cast `GridironCharacter` (`self.GetAvatarActorFromActorInfo`) :!pure true))
  (`self.K2_HasAuthority`
    (:`True`
      (bind _asgridiron_character_2 (cast `GridironCharacter` OtherActor))
      (`GameplayStatics.ApplyPointDamage` _asgridiron_character_2 1500.0 _impactnormal Hit (`Pawn.GetController` _asgridiron_character) _asgridiron_character "/Game/Game/Abilities/Character/BP_DashDamageType.BP_DashDamageType_C")
      (`Character.LaunchCharacter` _asgridiron_character_2 (`KismetMathLibrary.MakeVector` (* (.x _impactnormal) -750.0) (* (.y _impactnormal) -750.0) 300.0) true true))))