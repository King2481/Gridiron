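; GA_Zoom is a weapon gameplay ability that makes a GridironCharacter aim down with a zoomed camera while the input is held.
; On activation it commits, then starts aiming and waits for input release, which stops aiming and ends the ability.
; HandleAiming sets the character's aiming flag and switches its desired FOV between a narrow zoomed value and the normal one.
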(event `self.K2_ActivateAbility`
  (bind _returnvalue (`self.K2_CommitAbility`))
  (if _returnvalue
    (`AbilityTask_WaitInputRelease.WaitInputRelease` false
      (:`then`
        (`self.HandleAiming` true))
      (:`OnRelease`
        (`self.HandleAiming` false)
        (`self.K2_EndAbility`)))))

(fn `HandleAiming`
  (params (NewAim :type Boolean))
  (bind _asgridiron_character (cast `GridironCharacter` (`self.GetAvatarActorFromActorInfo`)))
  (`GridironCharacter.SetIsAiming` _asgridiron_character NewAim)
  (`GridironCharacter.SetDesiredFOV` _asgridiron_character (`KismetMathLibrary.SelectFloat` 50.0 90.0 NewAim)))