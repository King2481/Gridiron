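; Gameplay ability for the Quad Damage powerup, which grants GE_QuadDamage to the avatar character for a fixed duration.
; On successful commit it applies the effect, fades in a faint client-side screen tint and starts a timer that ends the ability.
; OnEndAbility clears the timer, removes all stacks of the effect, fades the tint out and plays a closing sound on the client.
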(event `self.K2_ActivateAbility`
  (bind _returnvalue (`self.K2_CommitAbility`))
  (if _returnvalue
    (`self.SetupQuad`)
    (bind _returnvalue_2 (`KismetSystemLibrary.K2_SetTimerDelegate` (delegate `OnQuadDamageEnded`) 20.0))
    (set `self.TimerHandle` _returnvalue_2)
    (else
      (`self.K2_EndAbility`))))

(event `OnQuadDamageEnded`
  (`self.K2_EndAbility`))

(event `self.K2_OnEndAbility`
  (params (bWasCancelled :type Boolean))
  (`KismetSystemLibrary.K2_ClearAndInvalidateTimerHandle` (`self.TimerHandle`))
  (bind _asgridiron_character (cast `GridironCharacter` (`self.GetAvatarActorFromActorInfo`)))
  (`|ExecutionSequence`
    (:`then_0`
      (`AbilitySystemComponent.RemoveActiveGameplayEffectBySourceEffect` (`GridironCharacter.AbilitySystemComponent` _asgridiron_character) "/Game/Game/Abilities/Powerups/GE_QuadDamage.GE_QuadDamage_C" null -1))
    (:`then_1`
      (bind _asgridiron_player_controller (cast `GridironPlayerController` (`Pawn.GetController` _asgridiron_character)))
      (`GridironPlayerController.ClientStartCameraFade` _asgridiron_player_controller 0.1 0.0 1.0 (`self.FadeOutColor`) false true)
      (`GridironPlayerController.ClientPlaySound2D` _asgridiron_player_controller "/Engine/VREditor/Sounds/VR_close_Cue.VR_close_Cue"))))

(fn `SetupQuad`
  (bind _asgridiron_character (cast `GridironCharacter` (`self.GetAvatarActorFromActorInfo`)))
  (`|ExecutionSequence`
    (:`then_0`
      (bind _asgridiron_player_controller (cast `GridironPlayerController` (`Pawn.GetController` _asgridiron_character)))
      (`GridironPlayerController.ClientStartCameraFade` _asgridiron_player_controller 0.0 0.1 1.0 (`self.FadeInColor`) false true))
    (:`then_2`
      (`AbilitySystemComponent.BP_ApplyGameplayEffectToSelf` :`self` (`GridironCharacter.AbilitySystemComponent` _asgridiron_character) :`GameplayEffectClass` "/Game/Game/Abilities/Powerups/GE_QuadDamage.GE_QuadDamage_C"))))