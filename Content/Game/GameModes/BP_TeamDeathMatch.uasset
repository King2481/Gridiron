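; Team deathmatch game mode for Gridiron that awards a team one point for each kill and decides the round winner.
; The kill event ignores self-kills and instigator-less deaths, scores through the GameState's team, and calls TeamWin once that team reaches ScoreNeededToWin.
; On timer expiry, it picks the first highest-scoring team, or calls Draw if none beats the starting high score, leaving the 255 sentinel ID.
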(event `self.BlueprintOnCharacterKilled`
  (params (Victim :type "GridironCharacter Object Reference") (KillingDamage :type "Float (single-precision)") (DamageEvent :type "DamageEvent Structure (by ref)") (EventInstigator :type "Controller Object Reference") (DamageCauser :type "Actor Object Reference"))
  (bind _playerstate (`Controller.PlayerState` EventInstigator))
  (bind _teamid (`GridironPlayerState.TeamId` (cast `GridironPlayerState` _playerstate :!pure true)))
  (`/Engine/EditorBlueprintResources/StandardMacros.IsValid` EventInstigator ; If the instigator was valid
    (:`Is Valid`
      (if (!= (`Pawn.PlayerState` Victim) _playerstate)
        (bind _asgridiron_game_state (cast `GridironGameState` (`GameplayStatics.GetGameState`)))
        (bind _returnvalue (`GridironGameState.GetTeamFromId` _asgridiron_game_state _teamid))
        (`/Engine/EditorBlueprintResources/StandardMacros.IsValid` _returnvalue
          (:`Is Valid`
            (`TeamInfo.ScorePoints` _returnvalue 1)
            (if (>= (`TeamInfo.TeamScore` _returnvalue) (`self.ScoreNeededToWin`))
              (`self.TeamWin` _teamid)))
          (:`Is Not Valid`
            (`KismetSystemLibrary.PrintString` (`KismetTextLibrary.Conv_TextToString` (`|FormatText` "Error: Team {TeamId} got a kill, but it is not in the gamestate" _teamid)) false)))))))

(fn `BlueprintOnRoundTimerExpired`
  (returns (ReturnValue :type Boolean))
  (locals (LocalGM :type "GridironGameModeBase Object Reference") (HighestTeamId :type Byte :default 255) (HighestTeamScore :type Integer))
  (bind _asgridiron_game_mode_base (cast `GridironGameModeBase` (`GameplayStatics.GetGameMode`))
    (:`then`
      (set `local.LocalGM` _asgridiron_game_mode_base)
      (bind _asgridiron_game_state (cast `GridironGameState` (`GameplayStatics.GetGameState`))
        (:`then`
          (for _array_element (`GridironGameState.Teams` _asgridiron_game_state)
            (bind _teamscore (`TeamInfo.TeamScore` _array_element))
            (if (> _teamscore (`local.HighestTeamScore`))
              (set `local.HighestTeamScore` _teamscore)
              (set `local.HighestTeamId` (`TeamInfo.TeamId` _array_element))))
          (if (!= (`local.HighestTeamId`) 255)
            (`self.TeamWin` (`local.LocalGM`) (`local.HighestTeamId`))
            (else
              (`self.Draw` (`local.LocalGM`))))
          (return true))
        (:`CastFailed`
          (`KismetSystemLibrary.PrintString` "ERR: Forcing a round end as the GameState is not valid in BP_Deathmatch")
          (return true))))
    (:`CastFailed`
      (`KismetSystemLibrary.PrintString` "ERR: Forcing a round end as the GameMode is not valid in BP_Deathmatch")
      (return true))))

(fn `UserConstructionScript`)